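; BP_Mobile is a Blueprint that sets up the mobile UI on the player's viewport when play begins.
; It takes the WBP_MobileUI instance from its Widget component, stores it and adds it to the viewport, rather than creating a new widget.
; It then switches the first player controller to UI-only input focused on that widget and shows the mouse cursor, printing an error if the cast fails.
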(event `self.ReceiveBeginPlay`
  ; Sets up the viewport for the player
  (bind _aswbp_mobile_ui (cast `/Game/Widgets/WBP_MobileUI` (`WidgetComponent.GetWidget` (`self.Widget`)))
    (:`then`
      (bind _output_get (set `self.WBP_MobileUI` _aswbp_mobile_ui))
      (`UserWidget.AddToViewport` _output_get 0)
      (`WidgetBlueprintLibrary.SetInputMode_UIOnlyEx` (`GameplayStatics.GetPlayerController` 0) (`self.WBP_MobileUI`))
      (set `PlayerController.bShowMouseCursor` true (`GameplayStatics.GetPlayerController` 0)))
    (:`CastFailed`
      (`KismetSystemLibrary.PrintString` "WBP_MobileIUI - Cast Failed" true true (struct :`R` 1.0 :`G` 1.0 :`A` 1.0) 15.0))))

(fn `UserConstructionScript`)