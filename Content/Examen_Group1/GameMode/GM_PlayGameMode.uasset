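; GM_PlayGameMode is a multiplayer game mode that gives each joining player a host or client pawn.
; PostLogin adds the controller to JoinedPlayers, spawning and possessing BP_Pawn_Host at index zero, otherwise BP_Pawn_Client.
; Client pawns receive that index as PlayerID and an RPCClientInitUI call at their shared spawn transform.
; OnLogout removes the controller from the array and destroys any pawn it still controls.
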(event `self.K2_PostLogin`
  (params (NewPlayer :type "PlayerController Object Reference"))
  ; When a player joins the session, creates the host or client pawn depending on if the host already exists
  (bind _returnvalue (`KismetArrayLibrary.Array_Add` (`self.JoinedPlayers`) NewPlayer))
  (if (== _returnvalue 0)
    (bind _returnvalue_2 (`|SpawnActorFromClass` "/Game/Examen_Group1/Blueprints/BP_Pawn_Host.BP_Pawn_Host_C" (`self.HostSpawnTransform`) "Undefined" "MultiplyWithRoot" null null))
    (`Controller.Possess` NewPlayer _returnvalue_2)
    (else
      (bind _returnvalue_3 (`|SpawnActorFromClass` "/Game/Examen_Group1/Blueprints/BP_Pawn_Client.BP_Pawn_Client_C" (`self.ClientSpawnTransform`) "Undefined" "MultiplyWithRoot" null _returnvalue null))
      (`Controller.Possess` NewPlayer _returnvalue_3)
      (`/Game/Examen_Group1/Blueprints/BP_Pawn_Client.RPC_Client_InitUI` _returnvalue_3))))

(event `self.K2_OnLogout`
  (params (ExitingController :type "Controller Object Reference"))
  (bind _returnvalue (`Controller.K2_GetPawn` ExitingController))
  ; Removes the player from the array when a player leaves the session, if the pawn is not automatically destroyed, destroys the pawn anyway
  (`KismetArrayLibrary.Array_RemoveItem` (`self.JoinedPlayers`) ExitingController)
  (`/Engine/EditorBlueprintResources/StandardMacros.IsValid` _returnvalue
    (:`Is Valid`
      (`self.K2_DestroyActor` _returnvalue))))

(fn `UserConstructionScript`)