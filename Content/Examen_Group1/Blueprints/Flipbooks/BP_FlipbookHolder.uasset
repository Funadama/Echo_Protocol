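; BP_FlipbookHolder is an actor that plays a one-shot Paper2D flipbook VFX from supplied data and start and end positions.
; It scales the play rate to fit the data's duration, then either moves along a location curve or snaps the flipbook to the end position.
; A second curve timeline drives scale, optionally mirroring X on the screen's right, then hides the flipbook and signals completion with itself as argument.
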(event `self.ReceiveBeginPlay`
  ; Disables the flipbook, turns the flipbook invisible and disables looping by default
  (`PaperFlipbookComponent.Stop` (`self.PaperFlipbook`))
  (`SceneComponent.SetVisibility` (`self.PaperFlipbook`) false false)
  (`PaperFlipbookComponent.SetLooping` (`self.PaperFlipbook`) false))

(event `PerformFlipbookVFX`
  (params (Data :type "/Game/Examen_Group1/Structs/S_VFX_FlipbookData Structure") (StartPosition :type "Vector Structure") (EndPosition :type "Vector Structure"))
  (bind _paperflipbook (`self.PaperFlipbook`))
  (bind ((`Flipbook_5_04C6C7024394D21D22C319A0CBDEEF6E` _flipbook)) (break `/Game/Examen_Group1/Structs/S_VFX_FlipbookData` (`self.Data`)))
  ; Starts the Flipbook VFX
  (set `self.Data` Data)
  (set `self.StartLocation` StartPosition)
  (set `self.EndLocation` EndPosition)
  (`/Engine/EditorBlueprintResources/StandardMacros.IsValid` _flipbook
    (:`Is Valid`
      (`PaperFlipbookComponent.SetFlipbook` (`self.PaperFlipbook`) _flipbook)
      (`SceneComponent.SetVisibility` (`self.PaperFlipbook`) true false)
      ;;[0 0 0 0.5] Scales the play rate of the animation to the duration
      (`PaperFlipbookComponent.SetPlayRate` _paperflipbook (/ (`PaperFlipbookComponent.GetFlipbookLength` _paperflipbook) (`.Duration_26_3B3E9C154B42028D345667A84D6F861B` (break `/Game/Examen_Group1/Structs/S_VFX_FlipbookData` (`self.Data`)))))
      (`PaperFlipbookComponent.PlayFromStart` (`self.PaperFlipbook`))
      (`self.HandleLocationChange`)
      (`self.StartScaleTimeline`))
    (:`Is Not Valid`
      (`KismetSystemLibrary.PrintString` "Invalid new flipbook"))))

(event `HandleLocationChange`
  (bind ((`LocationCurve_8_BF74118243C55D29524351A58850D09A` _locationcurve) (`Duration_26_3B3E9C154B42028D345667A84D6F861B` _duration)) (break `/Game/Examen_Group1/Structs/S_VFX_FlipbookData` (`self.Data`)))
  ; Handles the location change by either snapping the flipbook to the end location or lerping towards it using a timeline
  (if (`.ShouldVFXMove_14_837461424162EE6CC26E3C8E76EAEB1A` (break `/Game/Examen_Group1/Structs/S_VFX_FlipbookData` (`self.Data`)))
    (bind _value (`/Game/Examen_Group1/Libs/ML_Timeline.Timeline_FloatCurve` _locationcurve _duration :!via `PlayFromStart`)
      (:`Tick`
        (`self.K2_SetActorLocation` (`KismetMathLibrary.VLerp` (`self.StartLocation`) (`self.EndLocation`) _value))))
    (else
      (`SceneComponent.K2_SetWorldLocation` (`self.PaperFlipbook`) (`self.EndLocation`) false false))))

(event `StartScaleTimeline`
  (bind ((`ScaleCurve_11_AB00BF3A4A025E678E275E8EB9D9E550` _scalecurve) (`Duration_26_3B3E9C154B42028D345667A84D6F861B` _duration)) (break `/Game/Examen_Group1/Structs/S_VFX_FlipbookData` (`self.Data`)))
  ; Handles the scale change using a timeline
  (bind _value (`/Game/Examen_Group1/Libs/ML_Timeline.Timeline_FloatCurve` _scalecurve _duration :!via `PlayFromStart`)
    (:`Tick`
      (bind _returnvalue (`KismetMathLibrary.Conv_DoubleToVector` _value))
      (`self.SetActorScale3D` (`KismetMathLibrary.SelectVector` (`KismetMathLibrary.MakeVector` (* (.x _returnvalue) -1.0) (.y _returnvalue) (.z _returnvalue)) _returnvalue (and (`self.IsOnRightOfScreen`) (`.FlipWhenOnRight_22_61398AE046EAC168B91FD9B9E1CCD844` (break `/Game/Examen_Group1/Structs/S_VFX_FlipbookData` (`self.Data`)))))))
    (:`Completed`
      (`PaperFlipbookComponent.Stop` (`self.PaperFlipbook`))
      (`SceneComponent.SetVisibility` (`self.PaperFlipbook`) false false)
      (`self.OnFinishedVFX` self))))

(fn `UserConstructionScript`)