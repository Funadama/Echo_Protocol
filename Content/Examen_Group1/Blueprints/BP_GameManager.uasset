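; Game manager that runs a multiplayer turn-based fight between class-choosing clients and an enemy, overseen by a host.
; A server state machine cycles from Lobby through player turn, player action, enemy turn and enemy action, with placeholder random enemy input.
; Actions queue in maps and execute one-by-one through triggered loops advanced by completion dispatchers.
; It spawns pawns at array transforms drawn by the construction script, queuing players who join mid-action.
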(event `Server_BindSessionEvents`
  ;[0.149 0.149 0.149 0.502] Binds the events to the dispatchers of the GameMode
  (add `/Game/Examen_Group1/GameMode/GM_PlayGameMode.OnClientJoined` (`self.GameMode`) (`|CreateDelegate` :!event `RPC_Server_OnPlayerJoin`))
  (add `/Game/Examen_Group1/GameMode/GM_PlayGameMode.OnClientLeft` (`self.GameMode`) (`|CreateDelegate` :!event `Server_OnPlayerLeave`)))

(event `RPC_Server_ChangeGameState`
  (params (NewState :type "/Game/Examen_Group1/Enum/E_GameState Enum" :default "NewEnumerator0"))
  ; Changes the current active gameState
  (bind _output_get (set `self.CurrentState` NewState))
  (switch `/Game/Examen_Group1/Enum/E_GameState` _output_get
    (:`NewEnumerator1`
      (`self.Server_InitLobbyState`))
    (:`NewEnumerator2`
      (`self.Server_InitPlayerTurn`))
    (:`NewEnumerator3`
      (`self.Server_InitPlayerAction`))
    (:`NewEnumerator4`
      (`self.Server_InitEnemyTurn`))
    (:`NewEnumerator5`
      (`self.Server_InitEnemyAction`))))

(event `Server_InitLobbyState`
  ; Initiates the lobby state
)

(event `InitGameManager`
  (params (GameMode :type "/Game/Examen_Group1/GameMode/GM_PlayGameMode Object Reference"))
  ; Gets the GameManager ref, verifies the GameManager has enough spawnPoints for a full session and changes the gameState to Lobby
  (bind _output_get (set `self.GameMode` GameMode))
  (add `/Game/Examen_Group1/GameMode/GM_PlayGameMode.OnHostJoined` _output_get (`|CreateDelegate` :!event `SpawnHostPawn`))
  (bind _asgi_game_instance (cast `/Game/Examen_Group1/GameMode/GI_GameInstance` (`GameplayStatics.GetGameInstance`)))
  (`self.VerifySpawnPointCount` (`/Game/Examen_Group1/GameMode/GI_GameInstance.GetMaxPublicConnections` _asgi_game_instance))
  (`self.Server_BindSessionEvents`)
  (`self.RPC_Server_ChangeGameState` "NewEnumerator1"))

(event `SpawnHostPawn`
  (params (Controller :type "Controller Object Reference"))
  ; Spawns the host's pawn
  (bind _returnvalue (`|SpawnActorFromClass` "/Game/Examen_Group1/Blueprints/Pawns/BP_Pawn_Host.BP_Pawn_Host_C" (`|GetArrayItem` (`self.PawnSpawnLocations`)) "Undefined" "MultiplyWithRoot" null null))
  (`Controller.Possess` Controller _returnvalue)
  (`/Game/Examen_Group1/Blueprints/Pawns/BP_Pawn_Host.RPC_Server_InitHostUI` _returnvalue)
  (bind _hostui (`/Game/Examen_Group1/Blueprints/Pawns/BP_Pawn_Host.GetHostUI` _returnvalue))
  (set `self.HostUIWidget` _hostui))

(event `OnClientChoseClass`
  (params (PawnID :type Integer))
  ; Calls the dispatcher when the client has chosen their class
  (`/Game/Examen_Group1/Widgets/WBP_HostUI.InitPlayerHealthDisplay` (`self.HostUIWidget`) (`BlueprintMapLibrary.Map_Find` (`self.ClientPawns`) PawnID) "/Game/Examen_Group1/Widgets/WBP_EntityHealthBar_Mimi.WBP_EntityHealthBar_Mimi_C")
  (bind _canstart (`self.CanHostStartGame`))
  (`self.OnStartConditionsCheck` _canstart))

(event `VerifySpawnPointCount`
  (params (MaxConnections :type Integer))
  (bind _returnvalue (- (`KismetArrayLibrary.Array_Length` (`self.PawnSpawnLocations`)) 1))
  ; Checks to see if the max amount of connections possible for the session exceed the total amount of spawn points specified in the GameManager
  (if (> MaxConnections _returnvalue)
    (`KismetSystemLibrary.PrintText` (`|FormatText` "WARNING: More public connections [{MaxConnections}] possible than GameManager has available client spawnpoints [{ClientSpawnCount}]!" MaxConnections _returnvalue) true true (struct :`R` 1.0 :`G` 1.0 :`A` 1.0) 15.0)))

(event `RPC_Server_OnPlayerJoin`
  (params (Controller :type "Controller Object Reference") (ID :type Integer))
  ; Logic for when the player joins the session
  (switch `/Game/Examen_Group1/Enum/E_GameState` (`self.CurrentState`)
    (:`NewEnumerator1`
      ;;[0 0 0 0.5] Spawns in the client pawn, keeps the host from starting the game and waits on the new player to choose their class
      (bind _spawnedpawn (`self.SpawnClientPawn` Controller ID))
      (`BlueprintMapLibrary.Map_Add` (`self.ClientPawns`) ID _spawnedpawn)
      (add `/Game/Examen_Group1/Blueprints/Pawns/BP_Pawn_Client.OnClassChosen` _spawnedpawn (`|CreateDelegate` :!event `OnClientChoseClass`))
      (`self.OnStartConditionsCheck` false))
    (:`NewEnumerator2`
      ;;[0 0 0 0.5] Spawns in a client pawn and adds it to the action queue
      (bind _spawnedpawn_2 (`self.SpawnClientPawn` Controller ID))
      (`BlueprintMapLibrary.Map_Add` (`self.ClientPawns`) ID _spawnedpawn_2)
      (add `/Game/Examen_Group1/Blueprints/Pawns/BP_Pawn_Client.OnClassChosen` _spawnedpawn_2 (`|CreateDelegate` :!event `OnClientChoseClass_GameActive`)))
    (:`NewEnumerator3`
      ;;[0 0 0 0.5] Adds the joining player to a Queue that will be spawned upon the next PlayerInput state
      (`BlueprintMapLibrary.Map_Add` (`self.PlayerJoinQueue`) ID Controller :!label _label))
    (:`NewEnumerator4`
      (goto _label))
    (:`NewEnumerator5`
      (goto _label))))

(event `RPC_Client_PossessPawn`
  (params (Controller :type "Controller Object Reference") (Pawn :type "/Game/Examen_Group1/Blueprints/Pawns/BP_Pawn_Client Object Reference"))
  ; Has the client Possess the pawn
  (`Controller.Possess` Controller Pawn)
  (`/Game/Examen_Group1/Blueprints/Pawns/BP_Pawn_Client.RPC_Client_InitUI` Pawn))

(event `OnClientChoseClass_GameActive`
  (params (PawnID :type Integer))
  (bind _value (`BlueprintMapLibrary.Map_Find` (`self.ClientPawns`) PawnID))
  ; Spawns in the player healthbar when they choose their class
  (`self.Server_AddPawnToActionQueue` PawnID _value)
  (`/Game/Examen_Group1/Widgets/WBP_HostUI.InitPlayerHealthDisplay` (`self.HostUIWidget`) _value "/Game/Examen_Group1/Widgets/WBP_EntityHealthBar_Mimi.WBP_EntityHealthBar_Mimi_C"))

(event `RPC_Server_DestroyPawn`
  (params (Controller :type "Controller Object Reference") (ID :type Integer))
  (bind _value (`BlueprintMapLibrary.Map_Find` (`self.ClientPawns`) ID))
  ; Destroys the given pawn
  (`/Engine/EditorBlueprintResources/StandardMacros.IsValid` _value
    (:`Is Valid`
      (`self.K2_DestroyActor` _value))))

(event `RPC_Server_StartLobby`
  ; Unbinds the SessionEvents of the lobby and continues to the PlayerTurn state
  (if (`BlueprintMapLibrary.Map_IsNotEmpty` (`self.ClientPawns`))
    (`self.Server_BindSessionEvents`)
    (`/Game/Examen_Group1/Widgets/WBP_HostUI.InitEnemyHealthDisplay` (`self.HostUIWidget`) (`self.EnemyTarget`) "/Game/Examen_Group1/Widgets/WBP_EntityHealthBar_Enemy.WBP_EntityHealthBar_Enemy_C")
    (`self.RPC_Server_ChangeGameState` "NewEnumerator2")))

(event `Server_OnPlayerLeave`
  (params (Controller :type "Controller Object Reference") (ID :type Integer))
  ; Logic for when the player leaves the session
  (switch `/Game/Examen_Group1/Enum/E_GameState` (`self.CurrentState`)
    (:`NewEnumerator1`
      ;;[0 0 0 0.5] Removes the pawn from the ClientPawns map and checks if the host can start the game
      (`BlueprintMapLibrary.Map_Remove` (`self.ClientPawns`) ID)
      (bind _canstart (`self.CanHostStartGame`))
      (`self.OnStartConditionsCheck` _canstart))
    (:`NewEnumerator2`
      ;;[0 0 0 0.5] Removes the slot for the player from the PlayerActionQueue and resets everyone's selected actions to none
      (`BlueprintMapLibrary.Map_Remove` (`self.ClientPawns`) ID)
      (`BlueprintMapLibrary.Map_Remove` (`self.PlayerActionQueue`) ID)
      (`self.Server_NullifyInputQueue`))
    (:`NewEnumerator3`
      ;;[0 0 0 0.5] If the player has a valid pawn (is not in the joining queue), removes it's entries from the ClientPawns and PlayerActionQueue maps, also calls the dispatcher so the PerformPlayerActions event does not get stuck. Otherwise, it is simply removed from the PlayerJoinQueue
      (if (`.ReturnValue` (`BlueprintMapLibrary.Map_Find` (`self.ClientPawns`) ID)) :!label _label_2
        (`BlueprintMapLibrary.Map_Remove` (`self.PlayerActionQueue`) ID)
        (`BlueprintMapLibrary.Map_Remove` (`self.ClientPawns`) ID)
        (else
          (`BlueprintMapLibrary.Map_Remove` (`self.PlayerJoinQueue`) ID))))
    (:`NewEnumerator4`
      (goto _label_2))
    (:`NewEnumerator5`
      (goto _label_2))))

(event `Server_InitEnemyAction`
  ; Starts the EnemyAction state
  (`self.PerformEnemyActions`))

(event `Server_InitPlayerTurn`
  ; Initializes the input queue, binds to the dispatchers and enables the attack UI of the clients
  (if (not (`BlueprintMapLibrary.Map_IsEmpty` (`self.PlayerJoinQueue`)))
    (`self.Server_HandlePlayerJoinQueue`))
  (bind (_key _value) (`/Game/Examen_Group1/Libs/ML_Loops.ForEachLoop_Map` (`self.ClientPawns`))
    (:`Loop Body`
      ;;[0 0 0 0.5] Pawn is only added to queue if the owned entity is alive
      (bind _ownedentity (`/Game/Examen_Group1/Blueprints/Pawns/BP_Pawn_Client.OwnedEntity` _value)
        (:`then`
          (if (not (`/Game/Examen_Group1/Components/Health/Comp_EntityHealth.GetIsDead` (`/Game/Examen_Group1/Blueprints/Entities/BP_BaseEntity.Comp_EntityHealth` _ownedentity)))
            (`self.Server_AddPawnToActionQueue` _key _value)))
        (:`else`)))))

(event `Server_InitEnemyTurn`
  ; Starts the EnemyTurn state
  (`self.Server_GenerateEnemyInput`))

(event `Server_InitPlayerAction`
  ; Prepares for the client pawns to perform their chosen actions
  (bind (_key _value) (`/Game/Examen_Group1/Libs/ML_Loops.ForEachLoop_Map` (`self.ClientPawns`))
    (:`Loop Body`
      (`/Game/Examen_Group1/Blueprints/Pawns/BP_Pawn_Client.RPC_Client_ToggleAttackUI` _value false)
      (add `/Game/Examen_Group1/Blueprints/Pawns/BP_Pawn_Client.OnPawnDestroyed` _value (`|CreateDelegate` :!event `PlayerCompletedAction`)))
    (:`Completed`
      (`self.Server_PerformPlayerActions`))))

(event `PerformEnemyActions`
  ; Performs all Actions in the EnemyActionQueue one-by-one
  (bind (_key _value) (`/Game/Examen_Group1/Libs/ML_Loops.ForEachLoopWithTrigger_Map` (`self.EnemyActionQueue`) :!label _label_3)
    (:`Loop Body`
      (`KismetSystemLibrary.PrintText` (`|FormatText` "Enemy {EnemyID} started performing action {ActionID}" _key _value))
      (add `self.OnEnemyFinishedAction` (`|CreateDelegate` :!event `EnemyCompletedAction`))
      (`KismetSystemLibrary.Delay` (`self.TEMP_EnemyActionDuration`))
      (`self.OnEnemyFinishedAction`))
    (:`Completed`
      (`self.Server_ContinueToPlayerInput`))))

(event `Server_GenerateEnemyInput`
  ;[1 0.8987 0 0.5] Temporary solution to generate enemy attacks, will be replaced by actual AI later
  (for _index (range 1 (+ (`self.TEMP_EnemyActionCount`) 1))
    (`BlueprintMapLibrary.Map_Add` (`self.EnemyActionQueue`) _index (`KismetMathLibrary.RandomInteger` 10)))
  (`self.Server_ContinueToEnemyAction`))

(event `EnemyCompletedAction`
  ; Performs all Actions in the EnemyActionQueue one-by-one
  (remove `self.OnEnemyFinishedAction` (delegate `EnemyCompletedAction`))
  (`KismetSystemLibrary.PrintString` "Performed Enemy Action")
  (goto _label_3 :!via `Trigger`))

(event `Server_HandlePlayerJoinQueue`
  ; Handles spawning the player pawns if there are any waiting in the JoinQueue
  (bind (_key _value) (`/Game/Examen_Group1/Libs/ML_Loops.ForEachLoop_Map` (`self.PlayerJoinQueue`))
    (:`Loop Body`
      (`self.SpawnClientPawn` _value _key))))

(event `Server_PerformPlayerActions`
  ; Loops through all player actions one-by-one until every action is completed
  (bind (_key _value) (`/Game/Examen_Group1/Libs/ML_Loops.ForEachLoopWithTrigger_Map` (`self.PlayerActionQueue`) :!label _label_4)
    (:`Loop Body`
      (bind (_value_2 _returnvalue) (`BlueprintMapLibrary.Map_Find` (`self.ClientPawns`) _key))
      (if _returnvalue
        (add `/Game/Examen_Group1/Blueprints/Pawns/BP_Pawn_Client.OnPawnCompletedAction` _value_2 (`|CreateDelegate` :!event `PlayerCompletedAction`))
        (`/Game/Examen_Group1/Blueprints/Pawns/BP_Pawn_Client.Server_PerformActionOnEntity` _value_2 _value (`self.EnemyTarget`))
        (else
          ;;[1 1 0 0.5] Called when there's an invalid PlayerID
          (`KismetSystemLibrary.PrintText` (`|FormatText` "ERROR: Invalid PlayerID found! PlayerID: {ID}" _key) true true (struct :`R` 1.0 :`A` 1.0) 15.0))))
    (:`Completed`
      (`BlueprintMapLibrary.Map_Clear` (`self.PlayerActionQueue`))
      (`self.Server_ContinueToEnemyTurn`))))

(event `PlayerCompletedAction`
  (params (Pawn :type "/Game/Examen_Group1/Blueprints/Pawns/BP_Pawn_Client Object Reference"))
  ; Loops through all player actions one-by-one until every action is completed
  (remove `/Game/Examen_Group1/Blueprints/Pawns/BP_Pawn_Client.OnPawnCompletedAction` Pawn (delegate `PlayerCompletedAction`))
  (`KismetSystemLibrary.Delay` (`self.DelayBetweenPlayerAction`))
  (goto _label_4 :!via `Trigger`))

(event `Server_ContinueToPlayerInput`
  ; Clears the EnemyActionQueue and continues to the PlayerTurn state
  (`BlueprintMapLibrary.Map_Clear` (`self.EnemyActionQueue`))
  (`self.RPC_Server_ChangeGameState` "NewEnumerator2"))

(event `Server_AddPawnToActionQueue`
  (params (ID :type "Integer (by ref)") (Pawn :type "/Game/Examen_Group1/Blueprints/Pawns/BP_Pawn_Client Object Reference"))
  ; Adds the given pawn to the PlayerActionQueue
  (`BlueprintMapLibrary.Map_Add` (`self.PlayerActionQueue`) ID "NewEnumerator0")
  (add `/Game/Examen_Group1/Blueprints/Pawns/BP_Pawn_Client.OnUIActionSelected` Pawn (`|CreateDelegate` :!event `Server_QueueAction`))
  (add `/Game/Examen_Group1/Blueprints/Pawns/BP_Pawn_Client.OnUIActionCanceled` Pawn (`|CreateDelegate` :!event `Server_CancelAction`))
  (`/Game/Examen_Group1/Blueprints/Pawns/BP_Pawn_Client.RPC_Client_ToggleAttackUI` Pawn true))

(event `Server_ContinueToEnemyAction`
  ; Continues to the EnemyAction state
  (`self.RPC_Server_ChangeGameState` "NewEnumerator5"))

(event `Server_QueueAction`
  (params (PlayerID :type Integer) (Action :type "/Game/Examen_Group1/Enum/E_UIAction Enum" :default "NewEnumerator0"))
  ; Player Input
  (`BlueprintMapLibrary.Map_Add` (`self.PlayerActionQueue`) PlayerID Action)
  (bind _isallvalidinputs (`self.CheckActionQueue`))
  (if _isallvalidinputs
    (`self.Server_ContinueToPlayerAction`)))

(event `Server_ContinueToEnemyTurn`
  ; Continues to the EnemyInput state
  (bind (_key _value) (`/Game/Examen_Group1/Libs/ML_Loops.ForEachLoop_Map` (`self.ClientPawns`))
    (:`Loop Body`
      (`/Game/Examen_Group1/Blueprints/Pawns/BP_Pawn_Client.DisplayInputOnWidget` _value "NewEnumerator0"))
    (:`Completed`
      (`self.RPC_Server_ChangeGameState` "NewEnumerator4"))))

(event `Server_CancelAction`
  (params (PlayerID :type Integer))
  ; Player Input
  (`BlueprintMapLibrary.Map_Add` (`self.PlayerActionQueue`) PlayerID "NewEnumerator0"))

(event `Server_NullifyInputQueue`
  (bind _clientpawns (`self.ClientPawns`))
  ; Sets all the current actions to None
  (if (`BlueprintMapLibrary.Map_IsNotEmpty` _clientpawns)
    (bind (_key _value) (`/Game/Examen_Group1/Libs/ML_Loops.ForEachLoop_Map` _clientpawns)
      (:`Loop Body`
        (`self.Server_CancelAction` _key)
        (`/Game/Examen_Group1/Blueprints/Pawns/BP_Pawn_Client.DisplayInputOnWidget` _value "NewEnumerator0")
        (`/Game/Examen_Group1/Blueprints/Pawns/BP_Pawn_Client.RPC_Client_ToggleAttackUI` _value true)))))

(event `Server_ContinueToPlayerAction`
  ; Unbinds all events from PlayerInput dispatchers and clears the InputQueue
  (bind (_key _value) (`/Game/Examen_Group1/Libs/ML_Loops.ForEachLoop_Map` (`self.ClientPawns`))
    (:`Loop Body`
      (remove `/Game/Examen_Group1/Blueprints/Pawns/BP_Pawn_Client.OnUIActionSelected` _value (`|CreateDelegate` :!event `Server_QueueAction`))
      (remove `/Game/Examen_Group1/Blueprints/Pawns/BP_Pawn_Client.OnUIActionCanceled` _value (`|CreateDelegate` :!event `Server_CancelAction`)))
    (:`Completed`
      (`self.RPC_Server_ChangeGameState` "NewEnumerator3"))))

(fn `CanHostStartGame`
  (returns (CanStart :type Boolean))
  ; Returns true if there are clients in the lobby and all of them have chosen their class
  (if (`BlueprintMapLibrary.Map_IsEmpty` (`self.ClientPawns`))
    (return false)
    (else
      (bind (_key _value) (`/Game/Examen_Group1/Libs/ML_Loops.ForEachLoop_Map` (`self.ClientPawns`))
        (:`Loop Body`
          (`/Engine/EditorBlueprintResources/StandardMacros.IsValid` (`/Game/Examen_Group1/Blueprints/Pawns/BP_Pawn_Client.OwnedEntity` _value)
            (:`Is Not Valid`
              (return false))))
        (:`Completed`
          (return true))))))

(fn `CheckActionQueue`
  (returns (isAllValidInputs :type Boolean))
  ; Checks all values in the PlayerInput Queue map, if any of the values are not valid actions, returns false
  (bind _values (`BlueprintMapLibrary.Map_Values` (`self.PlayerActionQueue`)))
  (for _array_element _values
    (if (`|EnumEquality` _array_element "NewEnumerator0")
      (return false)))
  (return true))

(fn `DisplaySpawnTransforms`
  ; Display all transforms in the PawnSpawnLocations array. The host spawn is red, while the clients' are blue
  (`KismetSystemLibrary.FlushPersistentDebugLines`)
  (for (_array_element _array_index) (`self.PawnSpawnLocations`)
    (bind _returnvalue (* (.scale _array_element) (`self.DebugBoxExtentScale`)))
    (`KismetSystemLibrary.DrawDebugBox` (.location _array_element) _returnvalue (`KismetMathLibrary.SelectColor` (struct :`R` 1.0 :`A` 1.0) (struct :`B` 1.0 :`A` 1.0) (== _array_index 0)) (.rotation _array_element) (`self.DebugDrawDuration`))
    (`KismetSystemLibrary.DrawDebugArrow` (.location _array_element) (+ (.location _array_element) (* (`KismetMathLibrary.GetForwardVector` (.rotation _array_element)) (.x _returnvalue))) 5.0 (struct) (`self.DebugDrawDuration`) 5.0))
  (return))

(fn `SpawnClientPawn`
  (params (Controller :type "Controller Object Reference") (ID :type Integer))
  (returns (SpawnedPawn :type "/Game/Examen_Group1/Blueprints/Pawns/BP_Pawn_Client Object Reference"))
  ; Spawns in the client pawn and has the owning client possess it on their end
  (bind _returnvalue (`|SpawnActorFromClass` "/Game/Examen_Group1/Blueprints/Pawns/BP_Pawn_Client.BP_Pawn_Client_C" (`|GetArrayItem` (`self.PawnSpawnLocations`) ID) "Undefined" "MultiplyWithRoot" null ID null))
  (`self.RPC_Client_PossessPawn` (`local.Controller`) _returnvalue)
  (return _returnvalue))

(fn `UserConstructionScript`
  ; Displays the spawn transforms of the client and host pawns
  (if (not (`KismetSystemLibrary.IsPackagedForDistribution`))
    (`self.DisplaySpawnTransforms`)))