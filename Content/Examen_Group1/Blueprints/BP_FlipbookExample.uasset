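; Example actor that demonstrates and debugs flipbook VFX for combat actions on a skeletal mesh character.
; On BeginPlay it initializes the CompFlipbookVFX component with its mesh and which side of the screen it occupies.
; Per-action debug functions look up VFX data in a data asset and play it through the component.
; Stun, Ult, BasicAttack and Attack play on offensive targets, while Protect and Buff play on defensive targets.
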(event `self.ReceiveBeginPlay`
  ; Initiates the flipbookVFX component
  (`/Game/Examen_Group1/Components/VFX/Comp_FlipbookVFX.InitComponent` (`self.Comp_FlipbookVFX`) (`self.Entity Is on Right Of Screen`) (`self.SkeletalMesh`)))

(fn `Debug_PlayFlipbook_Attack`
  (`self.Debug_PlayFlipbook_Offense` "Attack"))

(fn `Debug_PlayFlipbook_Basic`
  (`self.Debug_PlayFlipbook_Offense` "BasicAttack"))

(fn `Debug_PlayFlipbook_Buff`
  (`self.Debug_PlayFlipbook_Defense` "Buff"))

(fn `Debug_PlayFlipbook_Defense`
  (params (Action :type Name))
  (`/Game/Examen_Group1/Components/VFX/Comp_FlipbookVFX.PlayFlipbookVFX` (`self.Comp_FlipbookVFX`) (`.VFXData_28_7151E62C4F3CDFBB731F9DBC0DB5A8C1` (break `/Game/Examen_Group1/Structs/S_ActionData` (`BlueprintMapLibrary.Map_Find` (`/Game/Examen_Group1/DataAssets/EntityActionData/PDA_ActionData_Base.ActionData` (`self.DataAsset`)) Action))) (`self.DefensiveTargets`)))

(fn `Debug_PlayFlipbook_Offense`
  (params (Action :type Name))
  (`/Game/Examen_Group1/Components/VFX/Comp_FlipbookVFX.PlayFlipbookVFX` (`self.Comp_FlipbookVFX`) (`.VFXData_28_7151E62C4F3CDFBB731F9DBC0DB5A8C1` (break `/Game/Examen_Group1/Structs/S_ActionData` (`BlueprintMapLibrary.Map_Find` (`/Game/Examen_Group1/DataAssets/EntityActionData/PDA_ActionData_Base.ActionData` (`self.DataAsset`)) Action))) (`self.OffensiveTargets`)))

(fn `Debug_PlayFlipbook_Protect`
  (`self.Debug_PlayFlipbook_Defense` "Protect"))

(fn `Debug_PlayFlipbook_Stun`
  (`self.Debug_PlayFlipbook_Offense` "Stun"))

(fn `Debug_PlayFlipbook_Ult`
  (`self.Debug_PlayFlipbook_Offense` "Ult"))

(fn `UserConstructionScript`)