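; Game instance that hosts and searches for LAN multiplayer sessions.
; CreateSession creates a session with a configurable connection limit, then opens the TEST_ServerHost level as a listen server on success.
; FindSessions searches the LAN up to a result cap, which a getter also exposes.
; Event dispatchers report success or failure of both operations, passing found sessions on for the UI to display.
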(event `CreateSession`
  ; Creates a session
  (`CreateSessionCallbackProxy.CreateSession` (`GameplayStatics.GetPlayerController` 0) (`self.MaxPublicConnections`) true
    (:`OnSuccess`
      (`KismetSystemLibrary.PrintString` "SUCCESS: Created lobby")
      (`self.OnCreatedLobby`)
      (`GameplayStatics.OpenLevelBySoftObjectPtr` "/Game/Examen_Group1/Maps/TEST_ServerHost.TEST_ServerHost" false "?listen"))
    (:`OnFailure`
      (`KismetSystemLibrary.PrintString` "ERROR: Failed to create lobby" true true (struct :`R` 1.0 :`A` 1.0) 15.0)
      (`self.OnFailedCreatingLobby`))))

(event `FindSessions`
  ; Finds all sessions on the current LAN and calls the dispatcher for the user interface to display them
  (bind _results (`FindSessionsCallbackProxy.FindSessions` (`GameplayStatics.GetPlayerController` 0) (`self.MaxSearchResults`) true true)
    (:`then`
      (`KismetSystemLibrary.PrintString` "Started searching"))
    (:`OnSuccess`
      (`self.OnFinishedGettingSessions` _results))
    (:`OnFailure`
      (`KismetSystemLibrary.PrintString` "Error, no sessions found")
      (`self.OnNoSessionsFound`))))

(fn `GetMaxSessionResults`
  (returns (MaxSearchResults :type Integer))
  ; Returns the max amount of session results
  (return (`self.MaxSearchResults`)))