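; Boss enemy Blueprint that picks a random action from its action data map, limited to those costing less than its current mana.
; Single-target actions defer to parent logic, while multi-target ones play their animation and spend mana, or finish immediately if the boss is stunned.
; Overridden perform and animation-finished events loop over targeted entities to apply damage and status effects, then trigger status behavior and return to idle.
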(event `self.StartAction`
  (params (Action :type Name) (TargetEntity :type "/Game/Examen_Group1/Blueprints/Entities/BP_BaseEntity Object Reference"))
  ; Chooses an action from the ActionDataMap before starting the action
  (bind (_chosenactionname _ismultitarget) (`self.ChooseAction`))
  (if _ismultitarget
    (`self.StartAction_MultiTarget` _chosenactionname)
    (else
      (`parent.StartAction` _chosenactionname TargetEntity))))

(event `StartAction_MultiTarget`
  (params (Action :type Name))
  ; Starts an action with multiple targets
  (bind _output_get (set `self.CurrentActionName` Action))
  ;;[0 0 0 0.5] Calls the dispatcher immediately if the entity is stunned
  (if (not (`/Game/Examen_Group1/Components/StatusEffects/Comp_StatusEffects.GetIsStunned` (`self.Comp_StatusEffects`)))
    (bind _output_get_2 (set `self.CurrentActionData` (`BlueprintMapLibrary.Map_Find` (`/Game/Examen_Group1/DataAssets/EntityActionData/PDA_ActionData_Base.ActionData` (`self.GetActionDataMap`)) (`self.CurrentActionName`))))
    (bind ((`Animation_17_2D91A7FD477FC2DC2E5FD88BA1D3BD53` _animation) (`ManaCost_23_E27571E04A3B2BBF4B2AE09EBBD0AC99` _manacost)) (break `/Game/Examen_Group1/Structs/S_ActionData` _output_get_2))
    (`self.PlayAnimation` _animation)
    (`/Game/Examen_Group1/Components/Mana/Comp_Mana.RemoveMana` (`self.Comp_Mana`) (`KismetMathLibrary.Conv_IntToDouble` _manacost))
    (else
      (`self.OnFinishedAction` _output_get))))

(event `/Game/Examen_Group1/Interfaces/BPI_Entity.Entity_PerformAction`
  (bind ((`Damage_10_0B71A52D4DDE84547641E99B5955D6F4` _damage) (`StatusEffects_19_2F8CFC5641CCEC53AE72CE96877B8D5E` _statuseffects)) (break `/Game/Examen_Group1/Structs/S_ActionData` (`self.CurrentActionData`)))
  ; Depending on if  the current action is multiTarget, performs the action on the chosen player entity or all player entities
  (if (`.IsMultiTarget_25_EAC288FE40B064CF287E3BBC3CD2EC6A` (break `/Game/Examen_Group1/Structs/S_ActionData` (`self.CurrentActionData`)))
    (bind _key (`/Game/Examen_Group1/Libs/ML_Loops.ForEachLoop_Map` (`self.TargetedEntities`))
      (:`Loop Body`
        (`self.TakeDamage` _key _damage)
        (`/Game/Examen_Group1/Components/StatusEffects/Comp_StatusEffects.AddStatusEffect` (`/Game/Examen_Group1/Blueprints/Entities/BP_BaseEntity.Comp_StatusEffects` _key) _statuseffects))
      (:`Completed`
        (`self.OnPerformAction` (`self.CurrentActionName`))))
    (else
      (`parent.Entity_PerformAction`))))

(event `/Game/Examen_Group1/Interfaces/BPI_Entity.Entity_AnimationFinished`
  ; Depending on if  the current action is multiTarget, uses the default AnimationFinished event or loops through the targeted entities to call TriggerStatusBehavior and return to the idle animation
  (if (`.IsMultiTarget_25_EAC288FE40B064CF287E3BBC3CD2EC6A` (break `/Game/Examen_Group1/Structs/S_ActionData` (`self.CurrentActionData`)))
    (bind _key (`/Game/Examen_Group1/Libs/ML_Loops.ForEachLoop_Map` (`self.TargetedEntities`))
      (:`Loop Body`
        (`/Game/Examen_Group1/Components/StatusEffects/Comp_StatusEffects.TriggerStatusBehavior` (`/Game/Examen_Group1/Blueprints/Entities/BP_BaseEntity.Comp_StatusEffects` _key) "NewEnumerator1"))
      (:`Completed`
        (`self.OnFinishedAction` (`self.CurrentActionName`))
        (`self.PlayAnimation` (`self.GetIdleAnimation`) true)))
    (else
      (`parent.Entity_AnimationFinished`))))

(fn `ChooseAction`
  (returns (ChosenActionName :type Name) (IsMultiTarget :type Boolean))
  (locals (L_ValidActions :type "Map of Name to /Game/Examen_Group1/Structs/S_ActionData Structure") (L_RandomIndex :type Integer :default 0))
  ; Checks which actions of the ActionDataMap are valid and returns a random valid action
  (bind (_key _value) (`/Game/Examen_Group1/Libs/ML_Loops.ForEachLoop_Map` (`/Game/Examen_Group1/DataAssets/EntityActionData/PDA_ActionData_Base.ActionData` (`self.GetActionDataMap`)))
    (:`Loop Body`
      (if (> (`KismetMathLibrary.FFloor` (`/Game/Examen_Group1/Components/Mana/Comp_Mana.GetCurrentMana` (`self.Comp_Mana`))) (`.ManaCost_23_E27571E04A3B2BBF4B2AE09EBBD0AC99` (break `/Game/Examen_Group1/Structs/S_ActionData` _value)))
        (`BlueprintMapLibrary.Map_Add` (`local.L_ValidActions`) _key _value)))
    (:`Completed`
      (set `local.L_RandomIndex` (`KismetMathLibrary.RandomInteger` (`BlueprintMapLibrary.Map_Length` (`local.L_ValidActions`))))
      (bind _keys (`BlueprintMapLibrary.Map_Keys` (`local.L_ValidActions`)))
      (bind _values (`BlueprintMapLibrary.Map_Values` (`local.L_ValidActions`)))
      (return (`|GetArrayItem` _keys (`local.L_RandomIndex`)) (`.IsMultiTarget_25_EAC288FE40B064CF287E3BBC3CD2EC6A` (break `/Game/Examen_Group1/Structs/S_ActionData` (`|GetArrayItem` _values (`local.L_RandomIndex`))))))))

(fn `UserConstructionScript`
  (`parent.UserConstructionScript`))