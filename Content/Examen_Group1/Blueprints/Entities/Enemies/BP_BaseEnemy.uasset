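; BP_BaseEnemy is a base enemy entity that reports when its action finishes and chooses whom to attack.
; On BeginPlay it binds to its finished-action event and re-broadcasts it as OnEnemyFinishedAction, mirroring the flow of player actions.
; The GetSmartTarget override filters players with CheckEntityHealthState and always returns an Attack on a random valid one.
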(event `self.ReceiveBeginPlay`
  ; Recall event to keep it similar to the player actions
  (`parent.ReceiveBeginPlay`)
  (add `self.OnFinishedAction` (delegate `OnFinishedAnimation_event`)))

(event `OnFinishedAnimation_event` :!signature `self.OnFinishedAction`
  (params (Action :type Name))
  ; Recall event to keep it similar to the player actions
  (`self.OnEnemyFinishedAction` self))

(fn `GetSmartTarget`
  (params (Players :type "Array of /Game/Examen_Group1/Blueprints/Entities/PlayableCharacters/BP_BaseCharacter Object Reference (by ref)"))
  (returns (Action :type Name) (Player :type "/Game/Examen_Group1/Blueprints/Entities/PlayableCharacters/BP_BaseCharacter Object Reference"))
  (locals (L_ValidPlayerTargets :type "Array of /Game/Examen_Group1/Blueprints/Entities/PlayableCharacters/BP_BaseCharacter Object Reference"))
  ; Override function for smart targeting
  (for _array_element Players
    (if (`/Game/Examen_Group1/Libs/FL_EntityChecks.CheckEntityHealthState` _array_element)
      (`KismetArrayLibrary.Array_Add` (`local.L_ValidPlayerTargets`) _array_element)))
  (return "Attack" (`KismetArrayLibrary.Array_Random` (`local.L_ValidPlayerTargets`))))

(fn `UserConstructionScript`
  (`parent.UserConstructionScript`))