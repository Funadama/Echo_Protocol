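; Base Blueprint for combat entities that perform named actions on a target, take damage and die.
; StartAction looks up the action in ActionDataMap and sends its animation to the AnimInstance through a message call.
; EntityPerformAction applies the action's damage to the target's health component, whose events trigger hurt or death animations.
; Dispatchers announce performed actions and finished animations, and idle resumes after any non-death animation.
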(event `self.ReceiveBeginPlay`
  ; Gets a reference to the animation instance, and binds events
  (set `self.AnimInstance` (`SkeletalMeshComponent.GetAnimInstance` (`self.SkeletalMesh`)))
  (`self.PlayAnimation` (`self.IdleAnimation`) true))

(event `StartAction`
  (params (Action :type Name) (TargetEnity :type "/Game/Examen_Group1/Blueprints/Entities/BP_BaseEntity Object Reference"))
  (bind (_value _returnvalue) (`BlueprintMapLibrary.Map_Find` (`self.ActionDataMap`) Action))
  ; Start animation
  (set `self.TargetEntity` TargetEnity)
  (set `self.CurrentActionName` Action)
  (if _returnvalue
    (bind _output_get (set `self.CurrentActionData` _value))
    (`self.PlayAnimation` (`.Animation_17_2D91A7FD477FC2DC2E5FD88BA1D3BD53` (break `/Game/Examen_Group1/Structs/S_ActionsData` _output_get)))
    (else
      (`KismetSystemLibrary.PrintText` (`|FormatText` "{Action} == Invalid (Did you configure ActionDataMap correctly?)" Action) true true (struct :`R` 1.0 :`G` 1.0 :`A` 1.0) 15.0))))

(event `PlayAnimation`
  (params (Animation :type "AnimationAsset Object Reference") (Looping :type Boolean))
  ; Play Animation
  (bind _animinstance (`self.AnimInstance`)
    (:`then`
      (set `self.CurrentAnimation` Animation)
      (message `/Game/Examen_Group1/Interfaces/BPI_EntityAnimation.EntityAnimation_PlayAnimation` _animinstance (`self.SkeletalMesh`) Animation Looping))
    (:`else`
      (`KismetSystemLibrary.PrintString` "Animation Instance invalid (Did you forget to call the parent BeginPlay node?)" true true (struct :`R` 1.0 :`G` 1.0 :`A` 1.0) 15.0))))

(event `/Game/Examen_Group1/Interfaces/BPI_Entity.Entity_PerformAction`
  ; Override function: prints which action was used
  (`KismetSystemLibrary.PrintText` (`|FormatText` "Performed: {Action} on {Target}" (`self.CurrentActionName`) (`KismetSystemLibrary.GetDisplayName` (`self.TargetEntity`))))
  (`self.TakeDamage` (`self.TargetEntity`) (`.Damage_10_0B71A52D4DDE84547641E99B5955D6F4` (break `/Game/Examen_Group1/Structs/S_ActionsData` (`self.CurrentActionData`))))
  (`self.OnPerformAction` (`self.CurrentActionName`)))

(event `/Game/Examen_Group1/Interfaces/BPI_Entity.Entity_AnimationFinished`
  ; Autoplay idle animation after an action
  (`self.OnFinishedAnimation` (`self.CurrentAnimation`))
  (if (and (!= (`self.CurrentAnimation`) (`self.IdleAnimation`)) (!= (`self.CurrentAnimation`) (`self.DeathAnimation`)))
    (`self.PlayAnimation` (`self.IdleAnimation`) true)))

(event `TakeDamage`
  (params (Damage :type Integer))
  ; Makes entity take damage
  (`/Game/Examen_Group1/Components/Health/Comp_EntityHealth.ApplyHealthChange` (`self.Comp_EntityHealth`) (* Damage -1)))

(event `self.Comp_EntityHealth.OnDeath`
  ; Handles health change animations
  ;;[0 0 0 0.5] Plays the death animation when the entity's health reaches 0
  (`self.PlayAnimation` (`self.DeathAnimation`)))

(event `self.Comp_EntityHealth.OnDamageTaken`
  (params (DamageTaken :type Integer))
  ; Handles health change animations
  ;;[0 0 0 0.5] Plays the hurt animation if the entity is damaged but not dead
  (if (not (`/Game/Examen_Group1/Components/Health/Comp_EntityHealth.GetIsDead` (`self.Comp_EntityHealth`)))
    (`self.PlayAnimation` (`self.HurtAnimation`))))

(fn `UserConstructionScript`)