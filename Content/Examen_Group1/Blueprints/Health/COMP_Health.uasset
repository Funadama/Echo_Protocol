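; Health component that tracks current and maximum health for its owning actor.
; SetHealth adds a signed amount clamped between zero and the maximum, firing OnHealthGained for positive amounts, otherwise OnDamageTaken, plus OnDeath when health is zero.
; SetMaxHealth shifts the maximum and passes the same amount to SetHealth so current health follows.
; ResetHealth refills to maximum without firing events.
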(fn `ResetHealth`
  ; Reset the health
  (set `self.CurrentHealth` (`self.MaxHealth`))
  (return))

(fn `SetHealth`
  (params (Amount :type Integer))
  ; Change the health
  (set `self.CurrentHealth` (`KismetMathLibrary.Clamp` (+ (`self.CurrentHealth`) (`local.Amount`)) 0 (`self.MaxHealth`)))
  ; When health changes send an event when health is gained or damage is taken
  (if (> (`local.Amount`) 0)
    (`self.OnHealthGained`)
    (return)
    (else
      (`self.OnDamageTaken`)
      ; Check if the health is 0 then call on death
      (if (== (`self.CurrentHealth`) 0)
        (`self.OnDeath`))
      (return))))

(fn `SetMaxHealth`
  (params (Amount :type Integer))
  ; Change the max health
  (set `self.MaxHealth` (+ (`self.MaxHealth`) Amount))
  ; Update current health so when max health is gained the current health doesn't stay te same
  (`self.SetHealth` (`local.Amount`)))