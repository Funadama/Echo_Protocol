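; BP_Pawn_Client is a client pawn that hosts a mobile UI and exposes client and server RPC events for it.
; The client init event creates WBP_MobileUI for player controller 0, adds it to the player screen and passes the pawn to its InitUI.
; The UI event handlers only print the button: the client one shows the button alone, while the server one adds the PlayerID.
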(event `RPC_Client_InitUI`
  ; Initiates the client's UI interface
  (bind _returnvalue (`|CreateWidget` "/Game/Examen_Group1/Widgets/WBP_MobileUI.WBP_MobileUI_C" (`GameplayStatics.GetPlayerController` 0)))
  (`UserWidget.AddToPlayerScreen` _returnvalue 0)
  (`/Game/Examen_Group1/Widgets/WBP_MobileUI.InitUI` _returnvalue self))

(event `RPC_Client_UIEvent`
  (params (Button :type "/Game/Examen_Group1/Enum/E_UIEvent Enum" :default "NewEnumerator0"))
  ; Prints the text of the pressed button on the client
  (`KismetSystemLibrary.PrintText` (`|FormatText` "UI Event: {Button}" (`|GenericToText` Button))))

(event `RPC_Server_UIEvent`
  (params (NewParam :type "/Game/Examen_Group1/Enum/E_UIEvent Enum" :default "NewEnumerator0"))
  ; Prints the text on the server stating the given UIEvent was called from which player
  (`KismetSystemLibrary.PrintText` (`|FormatText` "UI Event on Player {PlayerID}: {Button}" (`|GenericToText` NewParam) (`self.PlayerID`))))

(fn `UserConstructionScript`)